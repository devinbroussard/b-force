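; BP_MovingHazard is a moving hazard actor that turns its cube to follow its movement and plays a bounce sound on overlap.
; Each tick it smoothly interpolates the cube's world rotation toward the right vector of GetMovementDirection, which is defined outside this graph.
; Cube overlaps with actors of other classes play SC_BounceOff at the world origin, while overlaps with its own class are ignored.
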(event OnComponentBeginOverlap(Cube)
  (params (OverlappedComponent :type Primitive%20Component%20Object%20Reference) (OtherActor :type Actor%20Object%20Reference) (OtherComp :type Primitive%20Component%20Object%20Reference) (OtherBodyIndex :type Integer) (bFromSweep :type Boolean) (SweepResult :type Hit%20Result%20Structure%20%28by%20ref%29))
  (if (not (== (Utilities|GetClass OtherActor) (Utilities|GetClass self))) ; Checks if the other actor and self are from the smae class
    (Audio|PlaySoundatLocation "/Game/Sound/SC_BounceOff.SC_BounceOff" "0, 0, 0" "0, 0, 0" 1.0 1.0 0.0 0 0 0)))

(event EventBeginPlay)

(event Collision|EventActorBeginOverlap
  (params (OtherActor :type Actor%20Object%20Reference)))

(event EventTick
  (params (DeltaSeconds :type Float%20%28single-precision%29))
  (bind _returnvalue (Class|MovingHazard|GetMovementDirection))
  (Transformation|SetWorldRotation (Variables|Default|GetCube) (Math|Interpolation|RInterpTo (Transformation|GetWorldRotation (Variables|Default|GetCube)) (Math|Conversions|RotationFromXVector (Math|Vector|GetRightVector (Math|Rotator|MakeRotfromX _returnvalue))) DeltaSeconds 3.0) false false))

(fn ConstructionScript)