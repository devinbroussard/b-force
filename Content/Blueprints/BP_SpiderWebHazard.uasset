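; BP_SpiderWebHazard is a spider web hazard that plays a bounce reaction when the player touches it while unbroken.
; A collision mesh overlap from the player pawn plays a sound and writes the impact point to the PC_Data material parameter collection.
; A timeline curve scales the impact normal by an intensity value and writes it to the same collection, presumably driving material-based deformation rather than moving the player.
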(event OnComponentBeginOverlap(collisionMesh)
  (params (OverlappedComponent :type Primitive%20Component%20Object%20Reference) (OtherActor :type Actor%20Object%20Reference) (OtherComp :type Primitive%20Component%20Object%20Reference) (OtherBodyIndex :type Integer) (bFromSweep :type Boolean) (SweepResult :type Hit%20Result%20Structure%20%28by%20ref%29))
  (bind (_bblockinghit _binitialoverlap _time _distance _location _impactpoint _normal _impactnormal) (Collision|BreakHitResult SweepResult))
  (if (== OtherActor (Game|Player|GetPlayerPawn 0)) ; Checks if the player overlaps Mesh
    (bind _returnvalue (Class|SpiderWebHazard|GetIsBroken))
    (if (not _returnvalue) ; Checks if the spiderweb is broken
      (Audio|PlaySoundatLocation "/Game/Sound/SC_BounceOff.SC_BounceOff" (Transformation|GetActorLocation) "0, 0, 0" 1.0 1.0 0.0 0 0 0)
      (Rendering|Material|SetVectorParameterValue "/Game/Enviornments/Spiderwebs/Material/PC_Data.PC_Data" "Location" (Math|Conversions|ToLinearColor(Vector) _impactpoint) :!class /Script/Engine.KismetMaterialLibrary)
      (bind _cu_bounce (Timeline|BounceTimeLine PlayFromStart)
        (:Update
          (Rendering|Material|SetVectorParameterValue "/Game/Enviornments/Spiderwebs/Material/PC_Data.PC_Data" "Normal" (Math|Conversions|ToLinearColor(Vector) (* _impactnormal (* _cu_bounce (Variables|Default|GetIntenstity)))) :!class /Script/Engine.KismetMaterialLibrary))))))

(event EventBeginPlay)

(event EventTick
  (params (DeltaSeconds :type Float%20%28single-precision%29)))

(fn ConstructionScript)