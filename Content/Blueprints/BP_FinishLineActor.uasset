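; BP_FinishLineActor is a finish line whose two flower components display whether it is active.
; Every Tick it polls GetIsActive and sets both flowers to the active or inactive checkpoint material.
; When its Collider begins an overlap while active, it plays the lap completion sound at the world origin, without filtering the overlapping actor.
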(event OnComponentBeginOverlap(Collider)
  (params (OverlappedComponent :type Primitive%20Component%20Object%20Reference) (OtherActor :type Actor%20Object%20Reference) (OtherComp :type Primitive%20Component%20Object%20Reference) (OtherBodyIndex :type Integer) (bFromSweep :type Boolean) (SweepResult :type Hit%20Result%20Structure%20%28by%20ref%29))
  (bind _returnvalue (Class|CheckpointActor|GetIsActive))
  (if _returnvalue
    (Audio|PlaySoundatLocation "/Game/Sound/SC_LapCompletion.SC_LapCompletion" "0, 0, 0" "0, 0, 0" 1.0 1.0 0.0 0 0 0)))

(event EventBeginPlay)

(event Collision|EventActorBeginOverlap
  (params (OtherActor :type Actor%20Object%20Reference)))

(event EventTick
  (params (DeltaSeconds :type Float%20%28single-precision%29))
  (bind _flower (Variables|Default|GetFlower))
  (bind _flower2 (Variables|Default|GetFlower2))
  (bind _returnvalue (Class|CheckpointActor|GetIsActive))
  (if _returnvalue
    (Rendering|Material|SetMaterial _flower 0 "/Game/Enviornments/Track/Textures/MI_Checkpoint_Active.MI_Checkpoint_Active")
    (Rendering|Material|SetMaterial _flower2 0 "/Game/Enviornments/Track/Textures/MI_Checkpoint_Active.MI_Checkpoint_Active")
    (else
      (Rendering|Material|SetMaterial _flower 0 "/Game/Enviornments/Track/Textures/MI_Checkpoint_Inactive.MI_Checkpoint_Inactive")
      (Rendering|Material|SetMaterial _flower2 0 "/Game/Enviornments/Track/Textures/MI_Checkpoint_Inactive.MI_Checkpoint_Inactive"))))

(fn ConstructionScript)